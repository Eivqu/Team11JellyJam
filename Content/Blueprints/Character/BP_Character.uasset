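; Player character that toggles a security-camera-style tablet view from an input action.
; BeginPlay creates hidden tablet and static widgets; a FlipFlop on TabletToggle switches between the first CameraArray camera and the character's own view.
; Opening shows the cursor and tablet and blocks look and move input, closing reverses this, and both flash static briefly to mask the switch.
; Movement nodes are present but never run.
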(event `self.ReceiveBeginPlay`
  ;[1 1 1] Begin and create Widgets
  (`|ExecutionSequence`
    (:`then_0`
      (bind _returnvalue (`|CreateWidget` "/Game/Blueprints/UI/WBP_Tablet.WBP_Tablet_C"))
      (`UserWidget.AddToViewport` _returnvalue 0)
      (`Widget.SetVisibility` _returnvalue "Hidden"))
    (:`then_1`
      (bind _returnvalue_2 (`|CreateWidget` "/Game/Blueprints/UI/WBP_Static.WBP_Static_C"))
      (bind _output_get (set `self.StaticWidgetRef` _returnvalue_2))
      (`UserWidget.AddToViewport` _output_get 0)
      (`Widget.SetVisibility` _output_get "Hidden"))))

(event `InputAction|TabletToggle`
  (params (Key :type "Key Structure"))
  (bind _returnvalue (`GameplayStatics.GetPlayerController` 0))
  ;[1 1 1] Tablet Toggle function
  (:`Pressed`
    (`/Engine/EditorBlueprintResources/StandardMacros.FlipFlop`
      (:`A`
        (set `PlayerController.bShowMouseCursor` true _returnvalue)
        (`/Game/Blueprints/SecurityCamera/BP_SecurityCamera.SwitchToCamera` (`|GetArrayItem` (`self.CameraArray`)))
        (`Controller.SetIgnoreLookInput` _returnvalue true)
        (`Controller.SetIgnoreMoveInput` _returnvalue true)
        (`Widget.SetVisibility` (stale `self.ReceiveBeginPlay` _output_get) "Visible")
        (`KismetSystemLibrary.Delay` 0.1)
        (`Widget.SetVisibility` (stale `self.ReceiveBeginPlay` _output_get) "Hidden")
        (`Widget.SetVisibility` (stale `self.ReceiveBeginPlay` _returnvalue) "Visible"))
      (:`B`
        (set `PlayerController.bShowMouseCursor` false _returnvalue)
        (`PlayerController.SetViewTargetWithBlend` (`GameplayStatics.GetPlayerController` 0) self 0.0 "VTBlend_Linear" 0.0 false)
        (`Controller.SetIgnoreLookInput` _returnvalue false)
        (`Controller.SetIgnoreMoveInput` _returnvalue false)
        (`Widget.SetVisibility` (stale `self.ReceiveBeginPlay` _output_get) "Visible")
        (`KismetSystemLibrary.Delay` 0.1)
        (`Widget.SetVisibility` (stale `self.ReceiveBeginPlay` _output_get) "Hidden")
        (`Widget.SetVisibility` (stale `self.ReceiveBeginPlay` _returnvalue) "Hidden")))))

(fn `UserConstructionScript`)